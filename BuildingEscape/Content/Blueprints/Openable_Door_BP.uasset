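; Openable door actor that swings open and closed in response to the OnOpen and OnClose events of OpenDoor.
; The DoorSwing timeline plays forward to open and reverses to close, driving yaw from its OpenAngle curve.
; That yaw is combined with the rotation cached at BeginPlay, so the door works in any placed orientation.
; A timeline event track times the door lock sound at the actor's location.
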(event OnClose(OpenDoor)
  (bind _open_angle (Timeline|DoorSwing Reverse) ; Door swing
    (:Update
      (Transformation|SetActorRotation (Math|Rotator|CombineRotators (Math|Rotator|MakeRotator 0.0 0.0 _open_angle) (Variables|Default|GetinitialRotation))))
    (:Sound_Timing
      (Audio|PlaySoundatLocation "/Game/door-lock.door-lock" (Transformation|GetActorLocation)))))

(event OnOpen(OpenDoor)
  (bind _open_angle (Timeline|DoorSwing Play) ; Door swing
    (:Update
      (Transformation|SetActorRotation (Math|Rotator|CombineRotators (Math|Rotator|MakeRotator 0.0 0.0 _open_angle) (Variables|Default|GetinitialRotation))))
    (:Sound_Timing
      (Audio|PlaySoundatLocation "/Game/door-lock.door-lock" (Transformation|GetActorLocation)))))

(event EventBeginPlay
  (Variables|Default|SetinitialRotation (Transformation|GetActorRotation)) ; On event BeginPlay, get the Door object's rotation value so we can make a relative rotation off of that
)

(fn ConstructionScript)